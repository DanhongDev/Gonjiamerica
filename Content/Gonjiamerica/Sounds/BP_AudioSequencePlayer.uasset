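; Trigger-box audio player that plays two sounds in sequence, once triggered by the player character.
; The first box overlap starts NewSound1 and clears the Once flag.
; OnAudioFinished callbacks count replays up to FirstMaxCnt, switch to NewSound2, then count its replays against SecondMaxCnt.
; The first callback is never unbound, so it keeps restarting NewSound2 beyond that limit.
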(event `self.ReceiveBeginPlay`
  (bind _asmy_player_with_anim (cast `/Game/Gonjiamerica/Player/MyPlayerWithAnim` (`GameplayStatics.GetPlayerCharacter` 0)))
  (set `self.MyPlayer` _asmy_player_with_anim))

(event `self.Box.OnComponentBeginOverlap`
  (params (OverlappedComponent :type "PrimitiveComponent Object Reference") (OtherActor :type "Actor Object Reference") (OtherComp :type "PrimitiveComponent Object Reference") (OtherBodyIndex :type Integer) (bFromSweep :type Boolean) (SweepResult :type "HitResult Structure (by ref)"))
  (bind _audio (`self.Audio`))
  (if (`self.Once`)
    (if (== OtherActor (`self.MyPlayer`))
      (`AudioComponent.Stop` _audio)
      (`AudioComponent.SetSound` _audio (`self.New Sound_1`))
      (`AudioComponent.Play` _audio 0.0)
      (set `self.Once` false)
      (add `AudioComponent.OnAudioFinished` _audio (delegate `CheckFirstCnt`)))))

(event `CheckFirstCnt`
  (bind _audio (`self.Audio`))
  (bind _output_get (set `self.FirstPlayCnt` (+ (`self.FirstPlayCnt`) 1)))
  (if (<= _output_get (`self.FirstMaxCnt`))
    (`AudioComponent.Play` (`self.Audio`) 0.0)
    (else
      (`AudioComponent.Stop` _audio)
      (`AudioComponent.SetSound` _audio (`self.New Sound_2`))
      (`AudioComponent.Play` _audio 0.0)
      (add `AudioComponent.OnAudioFinished` _audio (delegate `CheckSecondCnt`)))))

(event `CheckSecondCnt`
  (bind _output_get (set `self.SecondPlayCnt` (+ (`self.SecondPlayCnt`) 1)))
  (if (<= _output_get (`self.SecondMaxCnt`))
    (`AudioComponent.Play` (`self.Audio`) 0.0)))

(fn `UserConstructionScript`)