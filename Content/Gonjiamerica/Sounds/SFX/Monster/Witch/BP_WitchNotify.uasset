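; Animation notify for the Witch monster that changes the sound playing on the animated mesh's owner.
; When fired, it finds the owner's AudioComponent, stops it, assigns the NewSound variable and restarts playback.
; An unconnected state switch leads to Idle, Run and Attack helpers that play Witch cues through the GameInstance's audio manager, so that path never runs.
; ChangeSound is an empty stub.
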(fn `AttackSound`
  (params (`Actor Location` :type "Vector Structure"))
  (bind _asbp_game_instance (cast `/Game/Gonjiamerica/SaveGame/BP_GameInstance` (`GameplayStatics.GetGameInstance`)))
  (`/Game/Gonjiamerica/Sounds/BP_AudioManager.PlaySFX` (`/Game/Gonjiamerica/SaveGame/BP_GameInstance.AudioManagerRef` _asbp_game_instance) "/Game/Gonjiamerica/Sounds/SFX/Monster/Witch/SC_WitchAttack.SC_WitchAttack" `Actor Location`))

(fn `Change Sound`
  (params (NewParam :type "Vector Structure") (NewParam1 :type "Vector Structure")))

(fn `IdleSound`
  (params (ActorLocation :type "Vector Structure"))
  (bind _asbp_game_instance (cast `/Game/Gonjiamerica/SaveGame/BP_GameInstance` (`GameplayStatics.GetGameInstance`)))
  (`/Game/Gonjiamerica/Sounds/BP_AudioManager.PlaySFX` (`/Game/Gonjiamerica/SaveGame/BP_GameInstance.AudioManagerRef` _asbp_game_instance) "/Game/Gonjiamerica/Sounds/SFX/Monster/Witch/SC_WitchCry.SC_WitchCry" ActorLocation))

(fn `Received_Notify`
  (params (MeshComp :type "SkeletalMeshComponent Object Reference") (Animation :type "AnimSequenceBase Object Reference") (EventReference :type "AnimNotifyEventReference Structure (by ref)"))
  (returns (ReturnValue :type Boolean))
  (bind _returnvalue (`Actor.GetComponentByClass` (`ActorComponent.GetOwner` MeshComp) "/Script/Engine.AudioComponent"))
  (`/Engine/EditorBlueprintResources/StandardMacros.IsValid` _returnvalue
    (:`Is Valid`
      (`AudioComponent.Stop` _returnvalue)
      (`AudioComponent.SetSound` _returnvalue (`self.New Sound`))
      (`AudioComponent.Play` _returnvalue 0.0))
    (:`Is Not Valid`
      _))
  (return false))

(fn `RunSound`
  (params (`Actor Location` :type "Vector Structure"))
  (bind _asbp_game_instance (cast `/Game/Gonjiamerica/SaveGame/BP_GameInstance` (`GameplayStatics.GetGameInstance`)))
  (`/Game/Gonjiamerica/Sounds/BP_AudioManager.PlaySFX` (`/Game/Gonjiamerica/SaveGame/BP_GameInstance.AudioManagerRef` _asbp_game_instance) "/Game/Gonjiamerica/Sounds/SFX/Monster/Witch/SC_WitchRun.SC_WitchRun" `Actor Location`))