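; Inventory component that holds item structs in ten slots and toggles an inventory widget with mouse cursor and input mode switching.
; AddItemToInventory casts the hit actor to BP_BaseItem, then puts it in the first slot that is empty or can stack it within the 64 limit.
; It then reloads the widget and destroys the actor, relying on the loop's IsValid check to skip remaining slots.
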(event `self.ReceiveBeginPlay`
  (bind _returnvalue (`|CreateWidget` "/Game/Gonjiamerica/Inventory/Widgets/WBP_Inentory.WBP_Inentory_C"))
  (set `self.Inventorywidget` _returnvalue)
  (`KismetArrayLibrary.Array_Resize` (`self.Items`) 10)
  (`/Game/Gonjiamerica/Inventory/Widgets/WBP_Inentory.LoadInventory` (`self.Inventorywidget`) self))

(event `EnhancedInput|/Game/Gonjiamerica/Player/Actions/IA_Inventory`
  (params (ActionValue :type Boolean) (ElapsedSeconds :type "Float (double-precision)") (TriggeredSeconds :type "Float (double-precision)") (InputAction :type "InputAction Object Reference" :default "/Game/Gonjiamerica/Player/Actions/IA_Inventory.IA_Inventory"))
  (bind _returnvalue (`GameplayStatics.GetPlayerController` 0))
  (bind _returnvalue_2 (`GameplayStatics.GetPlayerController` 0))
  (bind _inventorywidget (`self.Inventorywidget`))
  ;[1 1 1] Inventory Open/Close
  (:`Triggered`
    (if (`Widget.IsVisible` (`self.Inventorywidget`))
      (`Widget.RemoveFromParent` _inventorywidget)
      (set `PlayerController.bShowMouseCursor` false _returnvalue)
      (`WidgetBlueprintLibrary.SetInputMode_GameOnly` _returnvalue)
      (else
        (set `PlayerController.bShowMouseCursor` true _returnvalue_2)
        (`WidgetBlueprintLibrary.SetInputMode_GameAndUIEx` _returnvalue_2 null)
        (`UserWidget.AddToViewport` _inventorywidget 0)))))

(fn `AddItemToInventory`
  (params (`Hit Actor` :type "Actor Object Reference"))
  (bind _asbp_base_item (cast `/Game/Gonjiamerica/BluePrints/Items/BP_BaseItem` `Hit Actor`))
  (for (_array_element _array_index) (`self.Items`)
    (`/Engine/EditorBlueprintResources/StandardMacros.IsValid` _asbp_base_item
      (:`Is Valid`
        (bind (_name _description _stackable _quantity) (break `/Game/Gonjiamerica/Inventory/Blueprints/S_ItemStruct` _array_element))
        (bind (_name_2 _description_2 _stackable_2 _quantity_2) (break `/Game/Gonjiamerica/Inventory/Blueprints/S_ItemStruct` (`/Game/Gonjiamerica/BluePrints/Items/BP_BaseItem.Item` _asbp_base_item)))
        (bind _returnvalue (+ _quantity _quantity_2))
        (if (and (`KismetTextLibrary.EqualEqual_TextText` _name _name_2) _stackable_2 (<= _returnvalue 64))
          (bind (_item_name _item_description _item_stackable _item_quantity _item_mesh _item_scale _item_thumnail _item_inspectable) (break `/Game/Gonjiamerica/Inventory/Blueprints/S_ItemStruct` (`/Game/Gonjiamerica/BluePrints/Items/BP_BaseItem.Item` _asbp_base_item)))
          (`KismetArrayLibrary.Array_Set` (`self.Items`) _array_index (make `/Game/Gonjiamerica/Inventory/Blueprints/S_ItemStruct` _item_name _item_description _item_stackable _returnvalue _item_mesh (0.0 0.0 0.0) _item_thumnail _item_inspectable))
          (`/Game/Gonjiamerica/Inventory/Widgets/WBP_Inentory.LoadInventory` (`self.Inventorywidget`) self :!label _label)
          (`Actor.K2_DestroyActor` _asbp_base_item)
          (elif (== _quantity 0)
            (`KismetArrayLibrary.Array_Set` (`self.Items`) _array_index (`/Game/Gonjiamerica/BluePrints/Items/BP_BaseItem.Item` _asbp_base_item))
            (goto _label)))))))