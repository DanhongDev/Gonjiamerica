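; Interactive door that cycles through closed, partially open and fully open, swinging away from the interacting player.
; DoorInteract picks the swing side with a dot product and enables Tick-driven yaw interpolation toward the next position.
; A DoorSoundTime timer then stops movement and advances the state.
; A box overlap also briefly re-enables rotation after a delay, if the player's facing is off the world Y axis.
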(event `self.ReceiveBeginPlay`
  (bind _asmy_player_with_anim (cast `/Game/Gonjiamerica/Player/MyPlayerWithAnim` (`GameplayStatics.GetPlayerCharacter` 0)))
  (set `self.CharacterRef` _asmy_player_with_anim))

(event `self.ReceiveTick`
  (params (DeltaSeconds :type "Float (single-precision)"))
  (if (`self.bInteractWithDoor?`)
    (`self.HandleDoor`)))

(event `DoorInteract`
  (params (Player :type "/Game/Gonjiamerica/Player/MyPlayerWithAnim Object Reference"))
  ;[1 1 1] Door Interaction Mathmatics
  (if (> (`KismetMathLibrary.Dot_VectorVector` (`self.GetActorForwardVector` Player) (`SceneComponent.GetForwardVector` (`self.DoorOpenLocation`))) 0.0)
    (set `self.DoorOpenSide` 1.0)
    (else
      (set `self.DoorOpenSide` -1.0)))
  (set `self.bInteractWithDoor?` true)
  (`KismetSystemLibrary.K2_SetTimerDelegate` (delegate `SwitchDoorState`) (`self.DoorSoundTime`)))

(event `SwitchDoorState`
  ;[1 1 1] Door Interaction Mathmatics
  (set `self.bInteractWithDoor?` false)
  (switch `/Game/Gonjiamerica/BluePrints/Door/E_DoorState` (`self.E_DoorStates`)
    (:`NewEnumerator0`
      (set `self.E_DoorStates` "NewEnumerator1"))
    (:`NewEnumerator1`
      (set `self.E_DoorStates` "NewEnumerator2"))
    (:`NewEnumerator2`
      (set `self.E_DoorStates` "NewEnumerator0"))))

(event `HandleDoor`
  ;[1 1 1] Handle Door
  (switch `/Game/Gonjiamerica/BluePrints/Door/E_DoorState` (`self.E_DoorStates`)
    (:`NewEnumerator0`
      (`self.HandleRotation` (* (`self.DoorOpenSide`) 15.0)))
    (:`NewEnumerator1`
      (`self.HandleRotation` (* (`self.DoorOpenSide`) (`self.DoorOpenAngle`))))
    (:`NewEnumerator2`
      (`self.HandleRotation` 0.0))))

(event `HandleRotation`
  (params (SetRotation :type "Float (double-precision)"))
  ;[1 1 1] Handle Rotation
  (`SceneComponent.K2_SetRelativeRotation` (`self.Door`) (`KismetMathLibrary.MakeRotator` 0.0 0.0 (`KismetMathLibrary.FInterpTo` (.yaw (`SceneComponent.RelativeRotation` (`self.Door`))) SetRotation (`GameplayStatics.GetWorldDeltaSeconds`) (`self.Interp Speed`))) false false))

(event `self.Box.OnComponentBeginOverlap`
  (params (OverlappedComponent :type "PrimitiveComponent Object Reference") (OtherActor :type "Actor Object Reference") (OtherComp :type "PrimitiveComponent Object Reference") (OtherBodyIndex :type Integer) (bFromSweep :type Boolean) (SweepResult :type "HitResult Structure (by ref)"))
  (bind _returnvalue (`GameplayStatics.GetPlayerCharacter` 0))
  (bind (_returnvalue_x _returnvalue_y) (`KismetMathLibrary.BreakVector` (`self.GetActorForwardVector` _returnvalue)))
  (if (and (== OtherActor _returnvalue) (`KismetMathLibrary.BooleanNOR` (>= _returnvalue_y 0.7) (<= _returnvalue_y -0.7)))
    (`KismetSystemLibrary.Delay` 0.5)
    (set `self.bInteractWithDoor?` true)
    (`self.HandleRotation` 0.0)
    (`KismetSystemLibrary.Delay` 1.4)
    (set `self.bInteractWithDoor?` false)))

(fn `UserConstructionScript`)