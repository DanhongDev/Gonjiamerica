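; BP_NextLevel is a level-exit trigger actor that sends the player to the level referenced by its Level variable.
; When a MyPlayerWithAnim enters its Box, it calls BlinkIn on that character.
; It caches the player character at BeginPlay and polls its EndLevel flag every Tick, opening the level and clearing the flag once set.
; The level load depends only on that flag, not directly on the overlap.
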(event `self.ReceiveBeginPlay`
  (bind _asmy_player_with_anim (cast `/Game/Gonjiamerica/Player/MyPlayerWithAnim` (`GameplayStatics.GetPlayerCharacter` 0)))
  (set `self.player` _asmy_player_with_anim))

(event `self.ReceiveTick`
  (params (DeltaSeconds :type "Float (single-precision)"))
  (bind _player (`self.player`))
  (if (`/Game/Gonjiamerica/Player/MyPlayerWithAnim.EndLevel` _player)
    (`GameplayStatics.OpenLevelBySoftObjectPtr` (`self.Level`))
    (set `/Game/Gonjiamerica/Player/MyPlayerWithAnim.EndLevel` false _player)))

(event `self.Box.OnComponentBeginOverlap`
  (params (OverlappedComponent :type "PrimitiveComponent Object Reference") (OtherActor :type "Actor Object Reference") (OtherComp :type "PrimitiveComponent Object Reference") (OtherBodyIndex :type Integer) (bFromSweep :type Boolean) (SweepResult :type "HitResult Structure (by ref)"))
  (bind _asmy_player_with_anim (cast `/Game/Gonjiamerica/Player/MyPlayerWithAnim` OtherActor))
  (`/Game/Gonjiamerica/Player/MyPlayerWithAnim.Blink_In` _asmy_player_with_anim))

(fn `UserConstructionScript`)