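; Forest monster Blueprint that exposes its animated actions as custom events: crawl, jump, stand up and attack.
; Each event plays its matching montage on the Mesh component.
; Jump and attack fire the OnJumpEnd and OnAttackEnd dispatchers whether the montage completes or is interrupted, while crawl and stand up send no end notification.
; The file holds no logic that decides when these actions run.
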(event `self.ReceiveBeginPlay`)

(event `Crawl`
  ;[1 1 1] Custom Montage
  (`|PlayMontage` (`self.Mesh`) "/Game/Assets/Juhyun/ForestMonster/Animations/Montage_Crawl.Montage_Crawl"))

(event `MonsterJump`
  ;[1 1 1] Custom Montage
  (`|PlayMontage` (`self.Mesh`) "/Game/Assets/Juhyun/ForestMonster/Animations/Montage_Jump.Montage_Jump"
    (:`OnCompleted`
      _)
    (:`OnInterrupted`
      _))
  (`self.OnJumpEnd`))

(event `StandUp`
  ;[1 1 1] Custom Montage
  (`|PlayMontage` (`self.Mesh`) "/Game/Assets/Juhyun/ForestMonster/Animations/Montage_StandUp.Montage_StandUp"))

(event `Attack`
  ;[1 1 1] Custom Montage
  (`|PlayMontage` (`self.Mesh`) "/Game/Assets/Juhyun/ForestMonster/Animations/Montage_Attack.Montage_Attack"
    (:`OnCompleted`
      _)
    (:`OnInterrupted`
      _))
  (`self.OnAttackEnd`))

(fn `UserConstructionScript`)