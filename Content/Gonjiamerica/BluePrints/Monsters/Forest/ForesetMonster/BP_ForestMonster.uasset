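; BP_ForestMonster is the forest monster Blueprint, providing player proximity detection and montage-driven actions.
; Every tick it sets a chase-mode flag from its distance to the player and draws a debug sphere smaller than that detection range.
; Custom events play crawl, jump, stand-up, attack and sleeping-idle montages on the mesh.
; Jump, attack and idle call end dispatchers whether their montage completes or is interrupted.
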(event `self.ReceiveBeginPlay`)

(event `self.ReceiveTick`
  (params (DeltaSeconds :type "Float (single-precision)"))
  (`KismetSystemLibrary.DrawDebugSphere` (`self.K2_GetActorLocation`) 1500.0 12 (struct :`R` 0.989583 :`A` 1.0))
  (if (<= (`self.GetDistanceTo` (`GameplayStatics.GetPlayerCharacter` 0)) 2000.0)
    (set `self.IsChasePlayerMode` true)
    (else
      (set `self.IsChasePlayerMode` false))))

(event `Crawl`
  ;[1 1 1] Custom Montage
  (`|PlayMontage` (`self.Mesh`) "/Game/Assets/ForestMonster/Animations/Montage_Crawl.Montage_Crawl"))

(event `MonsterJump`
  ;[1 1 1] Custom Montage
  (`|PlayMontage` (`self.Mesh`) "/Game/Assets/ForestMonster/Animations/Montage_Jump.Montage_Jump"
    (:`OnCompleted`
      _)
    (:`OnInterrupted`
      _))
  (`self.OnJumpEnd`))

(event `StandUp`
  ;[1 1 1] Custom Montage
  (`|PlayMontage` (`self.Mesh`) "/Game/Assets/ForestMonster/Animations/Montage_StandUp.Montage_StandUp"))

(event `Attack`
  ;[1 1 1] Custom Montage
  (`|PlayMontage` (`self.Mesh`) "/Game/Assets/ForestMonster/Animations/Montage_Attack.Montage_Attack"
    (:`OnCompleted`
      _)
    (:`OnInterrupted`
      _))
  (`self.OnAttackEnd`))

(event `Idle`
  ;[1 1 1] Custom Montage
  (`|PlayMontage` (`self.Mesh`) "/Game/Assets/ForestMonster/Animations/Montage_SleepingIdle.Montage_SleepingIdle"
    (:`OnCompleted`
      _)
    (:`OnInterrupted`
      _))
  (`self.OnIdleEnd`))

(fn `UserConstructionScript`)