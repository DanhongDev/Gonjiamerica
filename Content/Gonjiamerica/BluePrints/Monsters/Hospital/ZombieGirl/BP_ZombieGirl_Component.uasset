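; Actor component for the hospital ZombieGirl monster, handling player proximity, damage reactions, death and montage playback.
; Tick draws a debug range sphere and, within range, notifies AIC_ZombieGirl and polls Life changes while running or attacking.
; Hits report damage events and interrupt run or attack montages; below the Life threshold, interrupting either flags death and stops the behavior tree.
; Action events play montages, firing matching dispatchers on completion or interruption.
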(event `self.ReceiveBeginPlay`
  (set `self.PreviousLife` (`self.Life`))
  (set `self.SkeletalMeshComponent` (`Actor.GetComponentByClass` (`self.GetOwner`) "/Script/Engine.SkeletalMeshComponent")))

(event `self.ReceiveTick`
  (params (DeltaSeconds :type "Float (single-precision)"))
  (bind _returnvalue (`GameplayStatics.GetPlayerCharacter` 0))
  (bind _returnvalue_2 (`self.GetOwner`))
  (bind _range (`self.Range`))
  (bind _returnvalue_3 (`SkeletalMeshComponent.GetAnimInstance` (`self.SkeletalMeshComponent`)))
  (bind _returnvalue_4 (`SkeletalMeshComponent.GetAnimInstance` (`self.SkeletalMeshComponent`)))
  (bind _returnvalue_5 (`SkeletalMeshComponent.GetAnimInstance` (`self.SkeletalMeshComponent`)))
  (`KismetSystemLibrary.DrawDebugSphere` (`Actor.K2_GetActorLocation` _returnvalue_2) _range 12 (struct :`R` 1.0 :`A` 1.0))
  (bind _output_get (set `self.IsCloseToPlayer` (<= (`Actor.GetDistanceTo` _returnvalue_2 (`GameplayStatics.GetPlayerCharacter` 0)) _range)))
  (if _output_get
    (bind _asaic_zombie_girl (cast `/Game/Gonjiamerica/BluePrints/Monsters/Hospital/ZombieGirl/AI/AIC_ZombieGirl` (`AIBlueprintHelperLibrary.GetAIController` _returnvalue_2)))
    (`/Game/Gonjiamerica/BluePrints/Monsters/Hospital/ZombieGirl/AI/AIC_ZombieGirl.IsCloseToPlayer_ZombieGirl` _asaic_zombie_girl)
    (set `self.IsRunToPlayer` (> (`KismetMathLibrary.VSize` (`Actor.GetVelocity` (`self.GetOwner`))) 1.0))
    (if (and (`self.IsRunToPlayer`) (!= (`self.Life`) (`self.PreviousLife`)))
      (set `self.IsDamageWhileRun` true)
      (set `self.PreviousLife` (`self.Life`) :!label _label)
      (if (< -150.0 (`self.Life`))
        (`AISense_Damage.ReportDamageEvent` (`self.GetOwner`) _returnvalue 0.0 (`Actor.K2_GetActorLocation` _returnvalue))
        (if (`AnimInstance.Montage_IsPlaying` _returnvalue_3 "/Game/Assets/Zombie03_Monster/Animations/MT_ZombieGirl_Attack.MT_ZombieGirl_Attack")
          (`AnimInstance.Montage_Stop` _returnvalue_3 0.2 "/Game/Assets/Zombie03_Monster/Animations/MT_ZombieGirl_Attack.MT_ZombieGirl_Attack")
          (set `self.IsDamagedWhilteAtk` true)
          (elif (`AnimInstance.Montage_IsPlaying` _returnvalue_4 "/Game/Assets/Zombie03_Monster/Animations/MT_ZombieGirl_Run.MT_ZombieGirl_Run")
            (`AnimInstance.Montage_Stop` _returnvalue_4 0.2 "/Game/Assets/Zombie03_Monster/Animations/MT_ZombieGirl_Run.MT_ZombieGirl_Run")
            (set `self.IsDamageWhileRun` true)))
        (elif (`AnimInstance.Montage_IsPlaying` _returnvalue_5 "/Game/Assets/Zombie03_Monster/Animations/MT_ZombieGirl_Run.MT_ZombieGirl_Run")
          (`AnimInstance.Montage_Stop` _returnvalue_5 0.2 "/Game/Assets/Zombie03_Monster/Animations/MT_ZombieGirl_Run.MT_ZombieGirl_Run")
          (set `self.IsDamagedWhilteAtk` true)
          (set `self.IsDeath` true :!label _label_2)
          (bind _asaic_zombie_girl_2 (cast `/Game/Gonjiamerica/BluePrints/Monsters/Hospital/ZombieGirl/AI/AIC_ZombieGirl` (`AIBlueprintHelperLibrary.GetAIController` (`self.GetOwner`))))
          (`/Game/Gonjiamerica/BluePrints/Monsters/Hospital/ZombieGirl/AI/AIC_ZombieGirl.BTStop_ZombieGirl` _asaic_zombie_girl_2)
          (elif (`AnimInstance.Montage_IsPlaying` (`SkeletalMeshComponent.GetAnimInstance` (`self.SkeletalMeshComponent`)) "/Game/Assets/Zombie03_Monster/Animations/MT_ZombieGirl_Attack.MT_ZombieGirl_Attack")
            (`AnimInstance.Montage_Stop` (`SkeletalMeshComponent.GetAnimInstance` (`self.SkeletalMeshComponent`)) 0.2 "/Game/Assets/Zombie03_Monster/Animations/MT_ZombieGirl_Attack.MT_ZombieGirl_Attack")
            (set `self.IsDamagedWhilteAtk` true)
            (goto _label_2))))
      (elif (and (`self.Is Attacking`) (!= (`self.Life`) (`self.PreviousLife`)))
        (set `self.IsDamagedWhilteAtk` true)
        (goto _label)))))

(event `ZombieGirlAttack`
  (`|PlayMontage` (`self.SkeletalMeshComponent`) "/Game/Assets/Zombie03_Monster/Animations/MT_ZombieGirl_Attack.MT_ZombieGirl_Attack"
    (:`OnCompleted`
      (`self.OnZombieGirlAttack` :!label _label_3))
    (:`OnInterrupted`
      (goto _label_3))
    (:`OnNotifyBegin`
      (`AnimInstance.Montage_Stop` (`SkeletalMeshComponent.GetAnimInstance` (`self.SkeletalMeshComponent`)) 0.2 "/Game/Assets/ForestMonster/Animations/MT_Attack.MT_Attack"))))

(event `ZombieGirl Run`
  (`|PlayMontage` (`self.SkeletalMeshComponent`) "/Game/Assets/Zombie03_Monster/Animations/MT_ZombieGirl_Run.MT_ZombieGirl_Run"
    (:`OnCompleted`
      _)
    (:`OnInterrupted`
      _))
  (`self.OnZombieGirlRun`))

(event `ZombieGirl Idle`
  (`|PlayMontage` (`self.SkeletalMeshComponent`) "/Game/Assets/Zombie03_Monster/Animations/MT_ZombieGirl_Idle.MT_ZombieGirl_Idle"
    (:`OnCompleted`
      _)
    (:`OnInterrupted`
      _))
  (`self.OnZombieGirlIdle`))

(event `ZombieGirl_Damaged`
  (`|PlayMontage` (`self.SkeletalMeshComponent`) "/Game/Assets/Zombie03_Monster/Animations/MT_ZombieGirl_Damaged.MT_ZombieGirl_Damaged"
    (:`OnCompleted`
      _)
    (:`OnInterrupted`
      _))
  (`self.OnZombieGirlDamaged`))

(event `ZombieGirl_Dead`
  (`|PlayMontage` (`self.SkeletalMeshComponent`) "/Game/Assets/Zombie03_Monster/Animations/MT_ZombieGirl_Dead.MT_ZombieGirl_Dead"
    (:`OnCompleted`
      _)
    (:`OnInterrupted`
      _))
  (`self.OnZombieGirlDead`))