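; BP_ZombieGirl is a hospital zombie girl monster whose attack damages the player.
; Begin and end trace events start and clear a looping 0.01-second timer that runs a sphere trace for Pawn objects between the StartTracePos and EndTracePos components.
; Any hit subtracts a fixed amount from the first player character's PlayerLife, without checking the hit actor, then stops tracing.
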(event `EndDamageTrace`
  (if (`KismetSystemLibrary.K2_IsValidTimerHandle` (stale `BeginDamageTrace` _returnvalue))
    (`KismetSystemLibrary.K2_ClearAndInvalidateTimerHandle` (stale `BeginDamageTrace` _returnvalue))))

(event `BeginDamageTrace`
  (bind _returnvalue (`KismetSystemLibrary.K2_SetTimerDelegate` (delegate `Damage Trace`) 0.01 true)))

(event `Damage Trace`
  (bind (_outhit _returnvalue) (`KismetSystemLibrary.SphereTraceSingleForObjects` (`SceneComponent.K2_GetComponentLocation` (`self.StartTracePos`)) (`SceneComponent.K2_GetComponentLocation` (`self.EndTracePos`)) 25.0 (`|MakeArray` "ObjectTypeQuery3" :!type "EObjectTypeQuery Enum")))
  (if _returnvalue
    (bind _asmy_player_with_anim (cast `/Game/Gonjiamerica/Player/MyPlayerWithAnim` (`GameplayStatics.GetPlayerCharacter` 0)))
    (set `/Game/Gonjiamerica/Player/MyPlayerWithAnim.PlayerLife` (- (`/Game/Gonjiamerica/Player/MyPlayerWithAnim.PlayerLife` _asmy_player_with_anim) 40.0) _asmy_player_with_anim)
    (`self.EndDamageTrace`)))

(event `/Game/Gonjiamerica/BluePrints/Monsters/Hospital/ZombieGirl/BPI_ZombieGirl_Damage.BeginZombieGirlTrace`
  (`self.BeginDamageTrace`))

(event `/Game/Gonjiamerica/BluePrints/Monsters/Hospital/ZombieGirl/BPI_ZombieGirl_Damage.EndZombieGirlTrace`
  (`self.EndDamageTrace`))

(fn `UserConstructionScript`)