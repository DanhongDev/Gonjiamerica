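; Hospital zombie enemy character that chases and melee-attacks the player, reacts to damage and dies.
; Tick alerts its AI controller when the player is near and polls Life changes to set hit or death flags, stop montages and report damage to AI perception.
; Run, attack and damaged events play montages and fire end dispatchers, while death stops the behavior tree.
; A looping timer sphere-traces during attacks and subtracts player life on a hit.
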(event `self.ReceiveBeginPlay`
  (set `self.PreviousLife` (`self.Life`))
  (set `self.InitPos` (`self.K2_GetActorLocation`)))

(event `self.ReceiveTick`
  (params (DeltaSeconds :type "Float (single-precision)"))
  (bind _returnvalue (`GameplayStatics.GetPlayerCharacter` 0))
  (bind _returnvalue_2 (`SkeletalMeshComponent.GetAnimInstance` (`self.Mesh`)))
  (bind _returnvalue_3 (`SkeletalMeshComponent.GetAnimInstance` (`self.Mesh`)))
  (bind _returnvalue_4 (`SkeletalMeshComponent.GetAnimInstance` (`self.Mesh`)))
  (`KismetSystemLibrary.PrintString` (`KismetStringLibrary.Conv_DoubleToString` (`KismetMathLibrary.VSize` (`self.GetVelocity`))))
  (`KismetSystemLibrary.PrintString` (`KismetStringLibrary.Conv_BoolToString` (`self.IsRunToPlayer`)))
  (bind _output_get (set `self.IsCloseToPlayer` (<= (`self.GetDistanceTo` (`GameplayStatics.GetPlayerCharacter` 0)) (`self.Range`))))
  (set `self.IsRunToPlayer` (> (`KismetMathLibrary.VSize` (`self.GetVelocity`)) 1.0))
  (if _output_get
    (bind _asaic_zombie_monster (cast `/Game/Gonjiamerica/BluePrints/Monsters/Hospital/ZombieMonster/AI/AIC_ZombieMonster` (`self.GetController`)))
    (`/Game/Gonjiamerica/BluePrints/Monsters/Hospital/ZombieMonster/AI/AIC_ZombieMonster.IsCloseToPlayer_ZombieMonster` _asaic_zombie_monster)
    (if (and (`self.IsRunToPlayer`) (!= (`self.Life`) (`self.PreviousLife`)))
      (set `self.IsDamageWhileRun` true)
      (set `self.PreviousLife` (`self.Life`) :!label _label)
      (if (< -50.0 (`self.Life`))
        (`AISense_Damage.ReportDamageEvent` self _returnvalue 0.0 (`self.K2_GetActorLocation` _returnvalue))
        (if (`AnimInstance.Montage_IsPlaying` _returnvalue_3 "/Game/Assets/ZombieMonster/Animations/MT_Zombie_Attack.MT_Zombie_Attack")
          (`AnimInstance.Montage_Stop` _returnvalue_3 0.2 "/Game/Assets/ZombieMonster/Animations/MT_Zombie_Attack.MT_Zombie_Attack")
          (set `self.IsDamagedWhilteAtk` true)
          (elif (`AnimInstance.Montage_IsPlaying` _returnvalue_2 "/Game/Assets/ZombieMonster/Animations/MT_Zombie_Run.MT_Zombie_Run")
            (`AnimInstance.Montage_Stop` _returnvalue_2 0.2 "/Game/Assets/ZombieMonster/Animations/MT_Zombie_Run.MT_Zombie_Run")
            (set `self.IsDamageWhileRun` true)
            (else
              (`AnimInstance.Montage_Stop` (`SkeletalMeshComponent.GetAnimInstance` (`self.Mesh`)) 0.2 "/Game/Assets/ZombieMonster/Animations/MT_Zombie_Idle.MT_Zombie_Idle"))))
        (else
          (set `self.IsDeath` true)
          (if (`AnimInstance.Montage_IsPlaying` _returnvalue_4 "/Game/Assets/ZombieMonster/Animations/MT_Zombie_Run.MT_Zombie_Run")
            (`AnimInstance.Montage_Stop` _returnvalue_4 0.2 "/Game/Assets/ZombieMonster/Animations/MT_Zombie_Run.MT_Zombie_Run")
            (set `self.IsDamageWhileRun` true)
            (set `self.IsDeath` true :!label _label_2)
            (elif (`AnimInstance.Montage_IsPlaying` (`SkeletalMeshComponent.GetAnimInstance` (`self.Mesh`)) "/Game/Assets/ZombieMonster/Animations/MT_Zombie_Attack.MT_Zombie_Attack")
              (`AnimInstance.Montage_Stop` (`SkeletalMeshComponent.GetAnimInstance` (`self.Mesh`)) 0.2 "/Game/Assets/ZombieMonster/Animations/MT_Zombie_Attack.MT_Zombie_Attack")
              (set `self.IsDamagedWhilteAtk` true)
              (goto _label_2)))))
      (elif (and (`self.Is Attacking`) (!= (`self.Life`) (`self.PreviousLife`)))
        (set `self.IsDamagedWhilteAtk` true)
        (goto _label)
        (else
          (if (!= (`self.Life`) (`self.PreviousLife`)) :!label _label_3
            (set `self.IsDamagedWhileIdle` true)
            (`KismetSystemLibrary.Delay` 0.9)
            (set `self.IsDamagedWhileIdle` false)
            (goto _label)))))
    (else
      (goto _label_3))))

(event `EndDamageTrace`
  (if (`KismetSystemLibrary.K2_IsValidTimerHandle` (stale `BeginDamageTrace` _returnvalue))
    (`KismetSystemLibrary.K2_ClearAndInvalidateTimerHandle` (stale `BeginDamageTrace` _returnvalue))))

(event `ZombieMonster_MeleeAttack`
  ;[1 1 1] MeleeAttack
  (`|PlayMontage` (`self.Mesh`) "/Game/Assets/ZombieMonster/Animations/MT_Zombie_Attack.MT_Zombie_Attack" 1.5
    (:`OnCompleted`
      _)
    (:`OnInterrupted`
      _))
  (`self.OnZombieMonsterMeleeAttackEnd`))

(event `BeginDamageTrace`
  (bind _returnvalue (`KismetSystemLibrary.K2_SetTimerDelegate` (delegate `Damage Trace`) 0.01 true)))

(event `ZombieMonster_Run`
  ;[1 1 1] Run
  (`|PlayMontage` (`self.Mesh`) "/Game/Assets/ZombieMonster/Animations/MT_Zombie_Run.MT_Zombie_Run"
    (:`OnCompleted`
      _)
    (:`OnInterrupted`
      _))
  (`self.OnZombieMonsterRunEnd`))

(event `Damage Trace`
  (bind (_outhit _returnvalue) (`KismetSystemLibrary.SphereTraceSingleForObjects` (`SceneComponent.K2_GetComponentLocation` (`self.StartTracePos`)) (`SceneComponent.K2_GetComponentLocation` (`self.EndTracePos`)) 25.0 (`|MakeArray` "ObjectTypeQuery3" :!type "EObjectTypeQuery Enum")))
  (if _returnvalue
    (bind _asmy_player_with_anim (cast `/Game/Gonjiamerica/Player/MyPlayerWithAnim` (`GameplayStatics.GetPlayerCharacter` 0)))
    (set `/Game/Gonjiamerica/Player/MyPlayerWithAnim.PlayerLife` (- (`/Game/Gonjiamerica/Player/MyPlayerWithAnim.PlayerLife` _asmy_player_with_anim) (`self.AttackDamage`)) _asmy_player_with_anim)
    (`KismetSystemLibrary.PrintString` "HitByZombie")
    (`self.EndDamageTrace`)))

(event `ZombieMosnter_Damaged`
  ;[1 1 1] Damaged
  (`|PlayMontage` (`self.Mesh`) "/Game/Assets/ZombieMonster/Animations/MT_Zombie_Damaged.MT_Zombie_Damaged" 1.5
    (:`OnCompleted`
      _)
    (:`OnInterrupted`
      _))
  (`self.OnZombieMonsterDamagedWhileAtk`))

(event `/Game/Gonjiamerica/BluePrints/Monsters/Hospital/ZombieMonster/BPI_Zombie_Damage.BeginZombieTrace`
  (`self.BeginDamageTrace`))

(event `ZombieMonster_Dead`
  ;[1 1 1] Dead
  (bind _asaic_zombie_monster (cast `/Game/Gonjiamerica/BluePrints/Monsters/Hospital/ZombieMonster/AI/AIC_ZombieMonster` (`AIBlueprintHelperLibrary.GetAIController` (`self.GetOwner` self))))
  (`/Game/Gonjiamerica/BluePrints/Monsters/Hospital/ZombieMonster/AI/AIC_ZombieMonster.BTSTOP_ZombieMonster` _asaic_zombie_monster))

(event `/Game/Gonjiamerica/BluePrints/Monsters/Hospital/ZombieMonster/BPI_Zombie_Damage.EndZombieTrace`
  (`self.EndDamageTrace`))

(fn `UserConstructionScript`)