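; BP_ProvokeMonster is a Hospital monster that plays run, attack, bite, damaged and death montages, firing dispatchers as they end.
; Tick flags movement and polls Life: changes report a damage event blaming the player to AI perception and interrupt attacks, while zero triggers death and destruction.
; Begin/EndProvokeTrace toggle a looping-timer melee sphere trace against Pawns, which only stops itself on a hit, without applying damage.
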(event `self.ReceiveTick`
  (params (DeltaSeconds :type "Float (single-precision)"))
  (bind _returnvalue (`GameplayStatics.GetPlayerCharacter` 0))
  (bind _returnvalue_2 (`SkeletalMeshComponent.GetAnimInstance` (`self.Mesh`)))
  (set `self.IsRunToPlayer` (> (`KismetMathLibrary.VSize` (`self.GetVelocity`)) 1.0))
  (if (!= (`self.Life`) (`self.PreviousLife`))
    (set `self.PreviousLife` (`self.Life`))
    (if (> (`self.Life`) 0.0)
      (`AISense_Damage.ReportDamageEvent` self _returnvalue 0.0 (`self.K2_GetActorLocation` _returnvalue))
      (`KismetSystemLibrary.PrintString` (`KismetStringLibrary.Conv_DoubleToString` (`self.Life`)))
      (if (`AnimInstance.Montage_IsPlaying` _returnvalue_2 "/Game/Assets/ProvokeMonster/Animations/MT_ProvokeMonster_Attack.MT_ProvokeMonster_Attack")
        (`AnimInstance.Montage_Stop` _returnvalue_2 0.2 "/Game/Assets/ProvokeMonster/Animations/MT_ProvokeMonster_Attack.MT_ProvokeMonster_Attack"))
      (else
        (set `self.IsDeath` true)
        (`AnimInstance.Montage_Stop` (`SkeletalMeshComponent.GetAnimInstance` (`self.Mesh`)) 0.2 "/Game/Assets/ProvokeMonster/Animations/MT_ProvokeMonster_Attack.MT_ProvokeMonster_Attack")
        (`self.ProvokeDead`)))))

(event `self.ReceiveBeginPlay`
  (set `self.PreviousLife` (`self.Life`)))

(event `ProvokeDamaged`
  (`|PlayMontage` (`self.Mesh`) "/Game/Assets/ProvokeMonster/Animations/MT_ProvokeMonster_Damaged.MT_ProvokeMonster_Damaged"
    (:`OnCompleted`
      _)
    (:`OnInterrupted`
      _))
  (`self.OnProvokeMonsterDamaged`))

(event `ProvokeDamagedDuringRunning`
  (`|PlayMontage` (`self.Mesh`) "/Game/Assets/ProvokeMonster/Animations/MT_ProvokeMonster_Damaged.MT_ProvokeMonster_Damaged"
    (:`OnCompleted`
      _)
    (:`OnInterrupted`
      _))
  (`self.OnProvokeMonsterDamagedDuringRunning`))

(event `ProvokeDead`
  (`|PlayMontage` (`self.Mesh`) "/Game/Assets/ProvokeMonster/Animations/MT_ProvokeMonster_Death.MT_ProvokeMonster_Death"
    (:`OnCompleted`
      _)
    (:`OnInterrupted`
      _))
  (`self.OnProvokeMonsterDead`)
  (`self.K2_DestroyActor`))

(event `ProvokeRun`
  (`|PlayMontage` (`self.Mesh`) "/Game/Assets/ProvokeMonster/Animations/MT_ProvokeMonster_Run.MT_ProvokeMonster_Run"
    (:`OnCompleted`
      _)
    (:`OnInterrupted`
      _))
  (`self.OnProvokeMonsterRunEnd`))

(event `ProvokeMonster_Attack`
  (set `self.IsAttacking` true)
  (`|PlayMontage` (`self.Mesh`) "/Game/Assets/ProvokeMonster/Animations/MT_ProvokeMonster_Attack.MT_ProvokeMonster_Attack"
    (:`OnCompleted`
      (set `self.IsAttacking` false :!label _label)
      (`self.OnProvokeMonsterAttackEnd`))
    (:`OnInterrupted`
      (goto _label))
    (:`OnNotifyBegin`
      (if (not (`self.IsAttacking`))
        (`AnimInstance.Montage_Stop` (`SkeletalMeshComponent.GetAnimInstance` (`self.Mesh`)) 0.2 "/Game/Assets/ProvokeMonster/Animations/MT_ProvokeMonster_Attack.MT_ProvokeMonster_Attack")
        (set `self.IsAttacking` false)))))

(event `ProvokeMonster_Bite`
  (`|PlayMontage` (`self.Mesh`) "/Game/Assets/ProvokeMonster/Animations/MT_ProvokeMonster_Bite.MT_ProvokeMonster_Bite"
    (:`OnCompleted`
      _)
    (:`OnInterrupted`
      _))
  (`self.OnProvokeMonsterBiteEnd`))

(event `EndDamageTrace`
  (if (`KismetSystemLibrary.K2_IsValidTimerHandle` (stale `BeginDamageTrace` _returnvalue))
    (`KismetSystemLibrary.K2_ClearAndInvalidateTimerHandle` (stale `BeginDamageTrace` _returnvalue))))

(event `BeginDamageTrace`
  (bind _returnvalue (`KismetSystemLibrary.K2_SetTimerDelegate` (delegate `Damage Trace`) 0.01 true)))

(event `Damage Trace`
  (bind (_outhit _returnvalue) (`KismetSystemLibrary.SphereTraceSingleForObjects` :`Start` (`SceneComponent.K2_GetComponentLocation` (`self.StartMeleeTracePos`)) :`End` (`SceneComponent.K2_GetComponentLocation` (`self.EndMeleeTracePos`)) :`Radius` 25.0 :`ObjectTypes` (`|MakeArray` "ObjectTypeQuery3" :!type "EObjectTypeQuery Enum") :`DrawDebugType` "ForDuration"))
  (if _returnvalue
    (`self.EndDamageTrace`)))

(event `/Game/Gonjiamerica/BluePrints/Monsters/Hospital/ProvokeMonster/BPI_Provoke_Damage.BeginProvokeTrace`
  (`self.BeginDamageTrace`))

(event `/Game/Gonjiamerica/BluePrints/Monsters/Hospital/ProvokeMonster/BPI_Provoke_Damage.EndProvokeTrace`
  (`self.EndDamageTrace`))

(fn `UserConstructionScript`)