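; Hospital running monster for a horror encounter, revealed when the player enters its trigger box and able to idle or sprint.
; Tick polls the trigger overlap to show the mesh and set the triggered flag.
; Run and IDLE events play montages and fire end dispatchers on completion or interruption.
; Run plays its scream directly through a macro, since the very fast sprint montage appears to skip sound notifies.
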(event `Run`
  ;[1 1 1] 너무 빨리 사라져서 애니메이션에 노티파이로는 재생이 안되는거 같음.
  (bind _audiomanagerref (`/Game/Gonjiamerica/BluePrints/Macros/M_CastToGameInstance.CastMacro`)
    (:`Output`
      (`/Game/Gonjiamerica/Sounds/BP_AudioManager.PlaySFX` _audiomanagerref "/Game/Gonjiamerica/Sounds/SFX/Monster/Running/SC_RunningScream.SC_RunningScream" (`self.K2_GetActorLocation`))
      (`|PlayMontage` (`self.Mesh`) "/Game/RunningMonsterByFab/Demo/Animations/MT_RunningMonster_Sprint.MT_RunningMonster_Sprint" 500.0
        (:`OnCompleted`
          _)
        (:`OnInterrupted`
          _))
      (set `self.IsRunning` true)
      (`self.OnRunEnd`))))

(event `IDLE`
  (`|PlayMontage` (`self.Mesh`) "/Game/RunningMonsterByFab/Demo/Animations/MT_RunningMonster_Idle.MT_RunningMonster_Idle"
    (:`OnCompleted`
      _)
    (:`OnInterrupted`
      _))
  (`self.OnIdelEnd`))

(event `self.ReceiveTick`
  (params (DeltaSeconds :type "Float (single-precision)"))
  (if (`self.IsOverlappingActor` (`self.triggerbox`) (`GameplayStatics.GetPlayerCharacter` 0))
    (`SceneComponent.SetVisibility` (`self.Mesh`) true false)
    (set `self.IsTriggerd` true)))

(fn `UserConstructionScript`)