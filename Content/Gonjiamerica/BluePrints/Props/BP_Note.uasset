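; BP_Note is a readable note prop that shows its text on screen when the Interact input fires.
; With AutoRead set, the AutoReadNode macro uses a FlipFlop to alternate between opening and closing the note.
; Opening creates a WBP_NoteTexts widget and freezes player movement and look, while closing removes it and restores both.
; The non-AutoRead Inspect path is an unfinished stub, with its spawn and read nodes left disconnected.
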(event `EnhancedInput|/Game/Gonjiamerica/Player/Movement/IA_Interact`
  (params (ActionValue :type Boolean) (ElapsedSeconds :type "Float (double-precision)") (TriggeredSeconds :type "Float (double-precision)") (InputAction :type "InputAction Object Reference" :default "/Game/Gonjiamerica/Player/Movement/IA_Interact.IA_Interact"))
  (bind _charactermovement (`Character.CharacterMovement` (`GameplayStatics.GetPlayerCharacter` 0)))
  (:`Triggered`
    (if (not (`self.bAutoRead`))
      (if (`self.bInspect`)
        _)
      (else
        (bind _isa (`/Engine/EditorBlueprintResources/StandardMacros.FlipFlop`)
          (:`A`
            (set `self.Is A` _isa)
            (bind _returnvalue (`|CreateWidget` "/Game/Gonjiamerica/Widgets/WBP_NoteTexts.WBP_NoteTexts_C" null (`self.NoteText`)))
            (bind _output_get (set `self.NoteWidgetReference` _returnvalue))
            (`UserWidget.AddToViewport` _output_get 0)
            (`CharacterMovementComponent.DisableMovement` (`Character.CharacterMovement` (`GameplayStatics.GetPlayerCharacter` 0)))
            (`Controller.SetIgnoreLookInput` (`GameplayStatics.GetPlayerController` 0) true)
            (`Widget.SetRenderOpacity` (`/Game/Gonjiamerica/Widgets/WBP_NoteTexts.NoteCanvasPanel` (`self.NoteWidgetReference`)) 1.0)
            (set `self.Is A` false))
          (:`B`
            (`Widget.SetRenderOpacity` (`/Game/Gonjiamerica/Widgets/WBP_NoteTexts.NoteCanvasPanel` (`self.NoteWidgetReference`)) 0.0)
            (`Widget.RemoveFromParent` _returnvalue)
            (`CharacterMovementComponent.SetMovementMode` _charactermovement (`CharacterMovementComponent.DefaultLandMovementMode` _charactermovement) 0)
            (`Controller.SetIgnoreLookInput` (`GameplayStatics.GetPlayerController` 0) false)
            (`KismetSystemLibrary.PrintString` "Hello")))))))

(fn `UserConstructionScript`)