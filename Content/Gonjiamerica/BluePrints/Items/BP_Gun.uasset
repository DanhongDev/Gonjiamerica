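; BP_Gun is a gun pickup that the player collects by pressing Interact.
; Box overlap, with no check on the overlapping actor, enables player input and shows a text prompt; end overlap reverses both.
; Interact casts the player to MyPlayerWithAnim, makes its existing WeaponMesh visible and destroys the pickup.
; Tick keeps the text rotated toward the player character.
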(event `self.ReceiveBeginPlay`)

(event `self.ReceiveTick`
  (params (DeltaSeconds :type "Float (single-precision)"))
  (`SceneComponent.K2_SetWorldRotation` (`self.TextRender`) (`KismetMathLibrary.FindLookAtRotation` (`SceneComponent.K2_GetComponentLocation` (`self.TextRender`)) (`self.K2_GetActorLocation` (`GameplayStatics.GetPlayerCharacter` 0))) false false))

(event `Obtain Gun`
  (bind _asmy_player_with_anim (cast `/Game/Gonjiamerica/Player/MyPlayerWithAnim` (`GameplayStatics.GetPlayerCharacter` 0)))
  (`SceneComponent.SetVisibility` (`/Game/Gonjiamerica/Player/MyPlayerWithAnim.weaponMesh` _asmy_player_with_anim) true false)
  (`self.K2_DestroyActor`))

(event `EnhancedInput|/Game/Gonjiamerica/Player/Actions/IA_Interact`
  (params (ActionValue :type Boolean) (ElapsedSeconds :type "Float (double-precision)") (TriggeredSeconds :type "Float (double-precision)") (InputAction :type "InputAction Object Reference" :default "/Game/Gonjiamerica/Player/Actions/IA_Interact.IA_Interact"))
  (:`Triggered`
    (`self.Obtain Gun`)))

(event `self.Box.OnComponentBeginOverlap`
  (params (OverlappedComponent :type "PrimitiveComponent Object Reference") (OtherActor :type "Actor Object Reference") (OtherComp :type "PrimitiveComponent Object Reference") (OtherBodyIndex :type Integer) (bFromSweep :type Boolean) (SweepResult :type "HitResult Structure (by ref)"))
  (`self.EnableInput` (`GameplayStatics.GetPlayerController` 0))
  (`SceneComponent.SetHiddenInGame` (`self.TextRender`) false false))

(event `self.Box.OnComponentEndOverlap`
  (params (OverlappedComponent :type "PrimitiveComponent Object Reference") (OtherActor :type "Actor Object Reference") (OtherComp :type "PrimitiveComponent Object Reference") (OtherBodyIndex :type Integer))
  (`self.DisableInput` (`GameplayStatics.GetPlayerController` 0))
  (`SceneComponent.SetHiddenInGame` (`self.TextRender`) true false))

(fn `UserConstructionScript`)