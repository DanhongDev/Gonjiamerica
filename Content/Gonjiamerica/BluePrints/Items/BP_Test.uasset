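; BP_Test is an interactable item that opens as a readable note and is consumed when the note closes.
; OnInteract shows a WBP_Note widget filled with the item's name and description, enables actor input, and swaps the IMC_GDCMotionMatching mapping context for IMC_Note.
; The IA_NoteUIClose action removes the widget, destroys the actor and restores the IMC_GDCMotionMatching context.
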(event `/Game/Gonjiamerica/BluePrints/Interfaces/BPI_Interact.On Interact`
  (params (Character :type "Object Object Reference"))
  (bind _returnvalue (`GameplayStatics.GetPlayerController` 0))
  (bind (_item_name _item_description) (break `/Game/Gonjiamerica/Inventory/Blueprints/S_ItemStruct` (`self.Item`)))
  (bind _returnvalue_2 (pcsubsystem `EnhancedInputLocalPlayerSubsystem` _returnvalue))
  ;[1 1 1] Interact
  (bind _returnvalue_3 (`|CreateWidget` "/Game/Gonjiamerica/BluePrints/Items/WBP_Note.WBP_Note_C" null _item_name _item_description))
  (bind _output_get (set `self.NoteWidget Ref` _returnvalue_3))
  (`UserWidget.AddToViewport` _output_get 0)
  (`self.EnableInput` _returnvalue)
  (`EnhancedInputSubsystemInterface.RemoveMappingContext` _returnvalue_2 "/Game/Gonjiamerica/Player/Actions/IMC_GDCMotionMatching.IMC_GDCMotionMatching" (struct))
  (`EnhancedInputSubsystemInterface.AddMappingContext` _returnvalue_2 "/Game/Gonjiamerica/Player/NoteActions/IMC_Note.IMC_Note" 0 (struct)))

(event `EnhancedInput|/Game/Gonjiamerica/Player/NoteActions/IA_NoteUIClose`
  (params (ActionValue :type Boolean) (ElapsedSeconds :type "Float (double-precision)") (TriggeredSeconds :type "Float (double-precision)") (InputAction :type "InputAction Object Reference" :default "/Game/Gonjiamerica/Player/NoteActions/IA_NoteUIClose.IA_NoteUIClose"))
  (bind _notewidget_ref (`self.NoteWidget Ref`))
  (bind _returnvalue (pcsubsystem `EnhancedInputLocalPlayerSubsystem` (`GameplayStatics.GetPlayerController` 0)))
  ;[1 1 1] Close NoteUI
  (:`Started`
    (`self.EnableInput` (`GameplayStatics.GetPlayerController` 0))
    (`/Engine/EditorBlueprintResources/StandardMacros.IsValid` _notewidget_ref
      (:`Is Valid`
        (`Widget.RemoveFromParent` _notewidget_ref)
        (set `self.NoteWidget Ref` null)
        (`self.K2_DestroyActor`)
        (`EnhancedInputSubsystemInterface.RemoveMappingContext` _returnvalue "/Game/Gonjiamerica/Player/NoteActions/IMC_Note.IMC_Note" (struct))
        (`EnhancedInputSubsystemInterface.AddMappingContext` _returnvalue "/Game/Gonjiamerica/Player/Actions/IMC_GDCMotionMatching.IMC_GDCMotionMatching" 0 (struct))))))

(fn `UserConstructionScript`
  (`parent.UserConstructionScript`))