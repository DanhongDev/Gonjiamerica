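; BP_LED1 is an LED light object whose two point lights flicker at random brightness.
; On BeginPlay it starts a looping timer, with an interval randomized once up to half a second, that rolls a new random Intensity.
; Tick pushes that value every frame to both lights as intensity and bloom scale.
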(event `self.ReceiveBeginPlay`
  (`KismetSystemLibrary.K2_SetTimerDelegate` (delegate `change intensity`) (`KismetMathLibrary.RandomFloatInRange` 0.0 0.5) true))

(event `change intensity`
  (set `self.intensity` (`KismetMathLibrary.RandomFloatInRange` 0.0 1000.0)))

(event `self.ReceiveTick`
  (params (DeltaSeconds :type "Float (single-precision)"))
  (bind _pointlight1 (`self.PointLight1`))
  (bind _intensity (`self.intensity`))
  (bind _pointlight (`self.PointLight`))
  (`LightComponent.SetIntensity` _pointlight1 _intensity)
  (`LightComponent.SetBloomScale` _pointlight1 _intensity)
  (`LightComponent.SetIntensity` _pointlight _intensity)
  (`LightComponent.SetBloomScale` _pointlight _intensity))

(fn `UserConstructionScript`)