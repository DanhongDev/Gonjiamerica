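; BP_BreakLamp is a lamp that breaks once when the player comes near it.
; While active, Tick compares the distance to player character 0 against Range rather than using overlap events.
; When triggered, it plays a crash sound, hides the PointLight, clears IsActive and applies a mass-independent force to Box toward the player, scaled by their separation.
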(event `self.ReceiveTick`
  (params (DeltaSeconds :type "Float (single-precision)"))
  (bind _returnvalue (`self.K2_GetActorLocation`))
  (bind _returnvalue_2 (- (`self.K2_GetActorLocation` (`GameplayStatics.GetPlayerCharacter` 0)) _returnvalue))
  (if (`self.isActive`)
    (if (<= (`KismetMathLibrary.VSize` _returnvalue_2) (`self.Range`))
      (`GameplayStatics.PlaySoundAtLocation` "/Game/Assets/Sounds/SFX/crash.crash" _returnvalue (struct) 0.5 1.0 0.0 null null null null)
      (`SceneComponent.SetVisibility` (`self.PointLight`) false false)
      (set `self.isActive` false)
      (`PrimitiveComponent.AddForce` (`self.Box`) (* _returnvalue_2 100.0) "None" true))))

(fn `UserConstructionScript`)