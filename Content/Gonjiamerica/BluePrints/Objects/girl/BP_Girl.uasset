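; BP_Girl is a scripted girl actor, apparently a scare, driven by a three-state Mode switch on Tick.
; She holds a tilted pose until ChangeMode starts her moving briefly along -X, then snaps her upright to GoalLocation.
; Once the player is close, she turns to face them, fires BlinkEvent on MyPlayerWithAnim, then destroys her trigger box and herself.
; Latent Delays inside Tick pace each stage.
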(event `self.ReceiveTick`
  (params (DeltaSeconds :type "Float (single-precision)"))
  (switch `int` (`self.mode`)
    (:`0`
      (`self.K2_SetActorRotation` (struct :`Yaw` -90.0 :`Roll` 30.0)))
    (:`1`
      (if (not (`self.Once`))
        (`self.AddMovementInput` (-10.0 0.0 0.0)))
      (`KismetSystemLibrary.Delay` 1.0)
      (`self.K2_SetActorLocation` (`self.GoalLocation`))
      (`self.K2_SetActorRotation` (struct :`Yaw` -90.0))
      (set `self.Once` true)
      (if (< (`self.GetDistanceTo` (`GameplayStatics.GetPlayerCharacter` 0)) 335.0)
        (set `self.mode` 2)))
    (:`2`
      (`self.K2_SetActorRotation` (`KismetMathLibrary.Conv_VectorToRotator` (- (`self.K2_GetActorLocation` (`GameplayStatics.GetPlayerCharacter` 0)) (`self.K2_GetActorLocation`))))
      (`KismetSystemLibrary.Delay` 1.0)
      (bind _asmy_player_with_anim (cast `/Game/Gonjiamerica/Player/MyPlayerWithAnim` (`GameplayStatics.GetPlayerCharacter` 0)))
      (`/Game/Gonjiamerica/Player/MyPlayerWithAnim.BlinkEvent` _asmy_player_with_anim)
      (`KismetSystemLibrary.Delay` 1.0)
      (`self.K2_DestroyActor` (`self.triggerbox`))
      (`self.K2_DestroyActor`))))

(event `ChangeMode`
  (set `self.mode` 1))

(fn `UserConstructionScript`)