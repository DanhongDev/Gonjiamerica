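; BP_Doll is a doll that, while Active, turns on yaw to face the player character every Tick.
; A dot-product test detects when the player's actor forward vector points within 30 degrees of it, then deactivates it and destroys its Triggerbox.
; A Bullet overlapping its Box while Active destroys both doll and Triggerbox.
; Nothing in this Blueprint sets Active to true.
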(event `self.ReceiveTick`
  (params (DeltaSeconds :type "Float (single-precision)"))
  (bind (_returnvalue_roll _returnvalue_pitch) (`KismetMathLibrary.BreakRotator` (`self.K2_GetActorRotation`)))
  (bind _returnvalue (`GameplayStatics.GetPlayerCharacter` 0))
  (bind (_returnvalue_roll_2 _returnvalue_pitch_2 _returnvalue_yaw) (`KismetMathLibrary.BreakRotator` (`KismetMathLibrary.MakeRotFromX` (- (`self.K2_GetActorLocation` (`GameplayStatics.GetPlayerCharacter` 0)) (`self.K2_GetActorLocation`)))))
  (if (`self.Active`)
    (`self.K2_SetActorRotation` (`KismetMathLibrary.MakeRotator` _returnvalue_roll _returnvalue_pitch _returnvalue_yaw))
    (if (>= (`KismetMathLibrary.Dot_VectorVector` (`KismetMathLibrary.Normal` (- (`self.K2_GetActorLocation`) (`self.K2_GetActorLocation` _returnvalue))) (`self.GetActorForwardVector` _returnvalue)) (`KismetMathLibrary.DegCos` 30.0))
      (set `self.Active` false)
      (`self.K2_DestroyActor` (`self.triggerbox`)))))

(event `self.Box.OnComponentBeginOverlap`
  (params (OverlappedComponent :type "PrimitiveComponent Object Reference") (OtherActor :type "Actor Object Reference") (OtherComp :type "PrimitiveComponent Object Reference") (OtherBodyIndex :type Integer) (bFromSweep :type Boolean) (SweepResult :type "HitResult Structure (by ref)"))
  (if (`GameplayStatics.ObjectIsA` OtherActor "/Game/Gonjiamerica/Player/Shot/Bullet.Bullet_C")
    (if (`self.Active`)
      (`self.K2_DestroyActor`)
      (`self.K2_DestroyActor` (`self.triggerbox`)))))

(fn `UserConstructionScript`)