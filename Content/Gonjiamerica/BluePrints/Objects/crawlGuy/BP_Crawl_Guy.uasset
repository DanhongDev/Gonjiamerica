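; Crawling character pawn that pursues the player once its Crawl flag is set, which nothing in this graph sets.
; While crawling, Tick unhides it, yaws it toward the player, snaps the mesh to the Updown transform and reissues AIMoveTo every frame.
; Otherwise the mesh is held at the Standard transform.
; Reaching the player destroys the referenced TriggerboxCantFlash and the pawn itself.
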(event `self.ReceiveTick`
  (params (DeltaSeconds :type "Float (single-precision)"))
  (bind (_returnvalue_roll _returnvalue_pitch) (`KismetMathLibrary.BreakRotator` (`self.K2_GetActorRotation`)))
  (bind (_returnvalue_location _returnvalue_rotation) (`KismetMathLibrary.BreakTransform` (`SceneComponent.GetRelativeTransform` (`self.standard`))))
  (bind (_returnvalue_roll_2 _returnvalue_pitch_2 _returnvalue_yaw) (`KismetMathLibrary.BreakRotator` (`KismetMathLibrary.MakeRotFromX` (- (`self.K2_GetActorLocation` (`GameplayStatics.GetPlayerCharacter` 0)) (`self.K2_GetActorLocation`)))))
  (if (`self.crawl`)
    (`self.SetActorHiddenInGame` false)
    (`self.K2_SetActorRotation` (`KismetMathLibrary.MakeRotator` _returnvalue_roll _returnvalue_pitch _returnvalue_yaw))
    (`self.FollowPlayer`)
    (else
      (`SceneComponent.K2_SetRelativeLocationAndRotation` (`self.Mesh`) _returnvalue_location _returnvalue_rotation false true))))

(event `FollowPlayer`
  (bind (_returnvalue_location _returnvalue_rotation) (`KismetMathLibrary.BreakTransform` (`SceneComponent.GetRelativeTransform` (`self.updown`))))
  (`SceneComponent.K2_SetRelativeLocationAndRotation` (`self.Mesh`) _returnvalue_location _returnvalue_rotation false false)
  (`|AIMoveTo` self (0.0 0.0 0.0) (`GameplayStatics.GetPlayerCharacter` 0) 100.0
    (:`OnSuccess`
      (`self.K2_DestroyActor` (`self.triggerboxCantFlash`))
      (`self.K2_DestroyActor`))))

(fn `UserConstructionScript`)