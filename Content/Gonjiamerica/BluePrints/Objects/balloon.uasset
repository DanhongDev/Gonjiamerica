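; Balloon actor that floats in place, turns to face the player and is destroyed when a Bullet overlaps it.
; Each Tick it bobs vertically on an incrementing sine angle and yaws toward player character 0.
; While the Active flag is set, it also drifts along world +X; nothing in this Blueprint sets that flag.
; Movement steps are per frame, without delta-time scaling.
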(event `self.ReceiveTick`
  (params (DeltaSeconds :type "Float (single-precision)"))
  (bind (_returnvalue_roll _returnvalue_pitch) (`KismetMathLibrary.BreakRotator` (`self.K2_GetActorRotation`)))
  (bind (_returnvalue_x _returnvalue_y _returnvalue_z) (`KismetMathLibrary.BreakVector` (`self.K2_GetActorLocation`)))
  (bind (_returnvalue_roll_2 _returnvalue_pitch_2 _returnvalue_yaw) (`KismetMathLibrary.BreakRotator` (`KismetMathLibrary.MakeRotFromX` (- (`self.K2_GetActorLocation` (`GameplayStatics.GetPlayerCharacter` 0)) (`self.K2_GetActorLocation`)))))
  (`self.K2_SetActorLocation` (`KismetMathLibrary.MakeVector` _returnvalue_x _returnvalue_y (+ _returnvalue_z (* (`KismetMathLibrary.DegSin` (`self.sin`)) 2.0))) true true)
  (set `self.sin` (+ (`self.sin`) 4.0))
  (`self.K2_SetActorRotation` (`KismetMathLibrary.MakeRotator` _returnvalue_roll _returnvalue_pitch _returnvalue_yaw))
  (if (`self.active`)
    (`self.K2_SetActorLocation` (+ (`self.K2_GetActorLocation`) (2.0 0.0 0.0)) true true)))

(event `self.ReceiveActorBeginOverlap`
  (params (OtherActor :type "Actor Object Reference"))
  (if (`GameplayStatics.ObjectIsA` OtherActor "/Game/Gonjiamerica/Player/Shot/Bullet.Bullet_C")
    (`self.K2_DestroyActor`)))

(fn `UserConstructionScript`)