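; BP_guys is a tilted actor that reacts to being seen by the player, then disappears.
; The RL flag picks the side it leans to, and it stays hidden until Active is set.
; Each Tick, a dot product against the player character's forward vector detects it within a view cone and plays a timeline.
; The timeline rolls it upright while yawing toward the player, then destroys it when finished.
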(event `self.ReceiveBeginPlay`
  (if (`self.RL`)
    (`self.K2_SetActorRotation` (struct :`Roll` 50.0))
    (else
      (`self.K2_SetActorRotation` (struct :`Roll` -50.0)))))

(event `self.ReceiveTick`
  (params (DeltaSeconds :type "Float (single-precision)"))
  (bind (_returnvalue_roll _returnvalue_pitch) (`KismetMathLibrary.BreakRotator` (`self.K2_GetActorRotation`)))
  (bind _returnvalue (`GameplayStatics.GetPlayerCharacter` 0))
  (bind (_returnvalue_roll_2 _returnvalue_pitch_2 _returnvalue_yaw) (`KismetMathLibrary.BreakRotator` (`KismetMathLibrary.MakeRotFromX` (- (`self.K2_GetActorLocation` (`GameplayStatics.GetPlayerCharacter` 0)) (`self.K2_GetActorLocation`)))))
  (if (`self.active`)
    (`self.SetActorHiddenInGame` false)
    (if (>= (`KismetMathLibrary.Dot_VectorVector` (`KismetMathLibrary.Normal` (- (`self.K2_GetActorLocation`) (`self.K2_GetActorLocation` _returnvalue))) (`self.GetActorForwardVector` _returnvalue)) (`KismetMathLibrary.DegCos` 50.0))
      (bind (_direction `_새_트랙_0`) (`Timeline|타임라인`)
        (:`Update`
          (if (`self.RL`)
            (`self.K2_SetActorRotation` (`KismetMathLibrary.MakeRotator` (`KismetMathLibrary.Lerp` 50.0 0.0 `_새_트랙_0`) _returnvalue_pitch _returnvalue_yaw))
            (else
              (`self.K2_SetActorRotation` (`KismetMathLibrary.MakeRotator` (`KismetMathLibrary.Lerp` -50.0 0.0 `_새_트랙_0`) _returnvalue_pitch _returnvalue_yaw)))))
        (:`Finished`
          (`self.K2_DestroyActor`))))
    (else
      (`self.SetActorHiddenInGame` true))))

(fn `UserConstructionScript`)