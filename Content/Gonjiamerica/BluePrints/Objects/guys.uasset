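; Placeable "guys" actor that swings through a pitch rotation and then removes itself once activated.
; BeginPlay sets a fixed starting rotation, and nothing more happens until the Active flag is true; this graph never sets that flag.
; While active, Tick applies Rot as pitch, raises it by a fixed per-frame step independent of delta time, and destroys the actor at an upper limit.
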(event `self.ReceiveBeginPlay`
  (`self.K2_SetActorRotation` (struct :`Pitch` -50.0)))

(event `self.ReceiveTick`
  (params (DeltaSeconds :type "Float (single-precision)"))
  (bind (_returnvalue_roll _returnvalue_pitch _returnvalue_yaw) (`KismetMathLibrary.BreakRotator` (`self.K2_GetActorRotation`)))
  (if (`self.active`)
    (`self.K2_SetActorRotation` (`KismetMathLibrary.MakeRotator` _returnvalue_roll (`self.rot`) _returnvalue_yaw))
    (set `self.rot` (+ (`self.rot`) 3.0))
    (if (>= (`self.rot`) 50.0)
      (`self.K2_DestroyActor`))))

(fn `UserConstructionScript`)