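; Interactive door actor that can be locked and cycles through closed, partially open and open each time HandleDoor fires.
; When locked, it searches the player's inventory component for an item matching UnlockKeyName, then clears that slot and refreshes the inventory widget.
; Without a key it plays a locked sound and shake timeline.
; Each state change plays its own sound and a timeline that drives the door's yaw.
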(event `HandleDoor`
  (bind _door (`self.Door`))
  (if (`self.isLocked?`)
    (bind _asmy_player_with_anim (cast `/Game/Gonjiamerica/Player/MyPlayerWithAnim` (`GameplayStatics.GetPlayerCharacter` 0)))
    (bind _returnvalue (`self.GetComponentByClass` _asmy_player_with_anim "/Game/Gonjiamerica/Inventory/Blueprints/BP_InventoryComponent.BP_InventoryComponent_C"))
    (bind _items (`/Game/Gonjiamerica/Inventory/Blueprints/BP_InventoryComponent.Items` _returnvalue))
    (for (_array_element _array_index) _items
      (if (`KismetTextLibrary.EqualEqual_TextText` (`self.UnlockKeyName`) (`.Name_2_45584B0D445A045E50FA6A82EB375022` (break `/Game/Gonjiamerica/Inventory/Blueprints/S_ItemStruct` _array_element)))
        (set `self.isLocked?` false)
        (bind _output_get (set `self.TargetIndex` _array_index))))
    (if (`self.isLocked?`)
      (bind _audiomanagerref (`/Game/Gonjiamerica/BluePrints/Macros/M_CastToGameInstance.CastMacro`)
        (:`Output`
          (`/Game/Gonjiamerica/Sounds/BP_AudioManager.PlaySFX` _audiomanagerref "/Game/Gonjiamerica/Sounds/SFX/Door/SC_LockedDoor.SC_LockedDoor" (`self.K2_GetActorLocation`))
          (bind (_direction _yawvalue) (`Timeline|Shake` :!via `PlayFromStart`)
            (:`Update`
              (`SceneComponent.K2_SetRelativeRotation` (`self.Door`) (`KismetMathLibrary.MakeRotator` 0.0 0.0 _yawvalue) false false)))))
      (else
        (`KismetArrayLibrary.Array_Set` _items _output_get (make `/Game/Gonjiamerica/Inventory/Blueprints/S_ItemStruct` "" "" false 0 null (0.0 0.0 0.0) null))
        (`/Game/Gonjiamerica/Inventory/Widgets/WBP_Inentory.LoadInventory` (`/Game/Gonjiamerica/Inventory/Blueprints/BP_InventoryComponent.Inventorywidget` _returnvalue) _returnvalue)
        (switch `/Game/Gonjiamerica/BluePrints/Objects/Door/E_DoorState` (`self.E_DoorStates`) :!label _label
          (:`NewEnumerator0`
            (set `self.E_DoorStates` "NewEnumerator1")
            (bind _audiomanagerref_2 (`/Game/Gonjiamerica/BluePrints/Macros/M_CastToGameInstance.CastMacro`)
              (:`Output`
                (`/Game/Gonjiamerica/Sounds/BP_AudioManager.PlaySFX` _audiomanagerref_2 "/Game/Gonjiamerica/Sounds/SFX/Door/SC_PartiallyOpen.SC_PartiallyOpen" (`self.K2_GetActorLocation`))
                (bind (_direction_2 _opendoor) (`Timeline|Partially Open` :!via `PlayFromStart`)
                  (:`Update`
                    (`SceneComponent.K2_SetRelativeRotation` _door (`KismetMathLibrary.MakeRotator` 0.0 0.0 _opendoor) false false))))))
          (:`NewEnumerator1`
            (set `self.E_DoorStates` "NewEnumerator2")
            (bind _audiomanagerref_3 (`/Game/Gonjiamerica/BluePrints/Macros/M_CastToGameInstance.CastMacro`)
              (:`Output`
                (`/Game/Gonjiamerica/Sounds/BP_AudioManager.PlaySFX` _audiomanagerref_3 "/Game/Gonjiamerica/Sounds/SFX/Door/SC_Open.SC_Open" (`self.K2_GetActorLocation`))
                (bind (_direction_3 _opendoor_2) (`Timeline|Open` :!via `PlayFromStart`)
                  (:`Update`
                    (`SceneComponent.K2_SetRelativeRotation` _door (`KismetMathLibrary.MakeRotator` 0.0 0.0 _opendoor_2) false false))))))
          (:`NewEnumerator2`
            (set `self.E_DoorStates` "NewEnumerator0")
            (bind _audiomanagerref_4 (`/Game/Gonjiamerica/BluePrints/Macros/M_CastToGameInstance.CastMacro`)
              (:`Output`
                (`/Game/Gonjiamerica/Sounds/BP_AudioManager.PlaySFX` _audiomanagerref_4 "/Game/Gonjiamerica/Sounds/SFX/Door/SC_Close.SC_Close" (`self.K2_GetActorLocation`))
                (bind (_direction_4 _opendoor_3) (`Timeline|Close` :!via `PlayFromStart`)
                  (:`Update`
                    (`SceneComponent.K2_SetRelativeRotation` _door (`KismetMathLibrary.MakeRotator` 0.0 0.0 _opendoor_3) false false)))))))))
    (else
      (goto _label))))

(fn `UserConstructionScript`)