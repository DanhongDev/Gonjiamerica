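; BP_StopSign is a stop sign prop that falls when the player character walks into its trigger box.
; An overlap by MyPlayerWithAnim calls Drop, which turns on physics simulation for the static mesh.
; After a one second delay, a flag lets the fall sound play only once at the sign's location.
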(event `Drop`
  (bind _staticmesh (`self.StaticMesh`))
  (`PrimitiveComponent.SetSimulatePhysics` _staticmesh true)
  (`KismetSystemLibrary.Delay` 1.0)
  (if (`self.Once`)
    (`GameplayStatics.PlaySoundAtLocation` "/Game/Gonjiamerica/Sounds/SFX/Environment/Forest/SC_SignFall.SC_SignFall" (`SceneComponent.K2_GetComponentLocation` _staticmesh) (struct) 1.0 1.0 0.0 null null null null)
    (set `self.Once` false)))

(event `self.Box.OnComponentBeginOverlap`
  (params (OverlappedComponent :type "PrimitiveComponent Object Reference") (OtherActor :type "Actor Object Reference") (OtherComp :type "PrimitiveComponent Object Reference") (OtherBodyIndex :type Integer) (bFromSweep :type Boolean) (SweepResult :type "HitResult Structure (by ref)"))
  (cast `/Game/Gonjiamerica/Player/MyPlayerWithAnim` OtherActor)
  (`self.Drop`))

(fn `UserConstructionScript`)