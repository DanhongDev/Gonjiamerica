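; Player inventory component that holds a ten-slot item array and displays it in an inventory widget.
; The inventory input toggles the widget, mouse cursor and input mode.
; Interact sphere-traces near the character's feet for a BP_Item, then scans slots in order, merging stackables up to 64 or filling an empty slot.
; A successful pickup reloads the widget and destroys the item, with the loop's validity check guarding later slots.
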(event `self.ReceiveBeginPlay`
  (bind _returnvalue (`|CreateWidget` "/Game/Gonjiamerica/Inventory/Widgets/WBP_Inentory.WBP_Inentory_C"))
  (set `self.Inventorywidget` _returnvalue)
  (`KismetArrayLibrary.Array_Resize` (`self.Itmes`) 10)
  (`/Game/Gonjiamerica/Inventory/Widgets/WBP_Inentory.LoadInventory` (`self.Inventorywidget`) self))

(event `EnhancedInput|/Game/Gonjiamerica/Player/Movement/IA_Inventory`
  (params (ActionValue :type Boolean) (ElapsedSeconds :type "Float (double-precision)") (TriggeredSeconds :type "Float (double-precision)") (InputAction :type "InputAction Object Reference" :default "/Game/Gonjiamerica/Player/Movement/IA_Inventory.IA_Inventory"))
  (bind _returnvalue (`GameplayStatics.GetPlayerController` 0))
  (bind _returnvalue_2 (`GameplayStatics.GetPlayerController` 0))
  (bind _inventorywidget (`self.Inventorywidget`))
  ;[1 1 1] Inventory Open/Close
  (:`Triggered`
    (if (`Widget.IsVisible` (`self.Inventorywidget`))
      (`Widget.RemoveFromParent` _inventorywidget)
      (set `PlayerController.bShowMouseCursor` false _returnvalue)
      (`WidgetBlueprintLibrary.SetInputMode_GameOnly` _returnvalue)
      (else
        (set `PlayerController.bShowMouseCursor` true _returnvalue_2)
        (`WidgetBlueprintLibrary.SetInputMode_GameAndUIEx` _returnvalue_2 null)
        (`UserWidget.AddToViewport` _inventorywidget 0)))))

(event `EnhancedInput|/Game/Gonjiamerica/Player/Movement/IA_Interact`
  (params (ActionValue :type Boolean) (ElapsedSeconds :type "Float (double-precision)") (TriggeredSeconds :type "Float (double-precision)") (InputAction :type "InputAction Object Reference" :default "/Game/Gonjiamerica/Player/Movement/IA_Interact.IA_Interact"))
  (bind _returnvalue (- (`Actor.K2_GetActorLocation` (`GameplayStatics.GetPlayerCharacter` 0)) (0.0 0.0 65.0)))
  ;[1 1 1] Obtain Items Logic
  (:`Triggered`
    (bind _outhit (`KismetSystemLibrary.SphereTraceSingle` _returnvalue _returnvalue 120.0 "TraceTypeQuery1"))
    (bind _asbp_item (cast `/Game/Gonjiamerica/Inventory/Blueprints/BP_Item` (`.HitActor` (`GameplayStatics.BreakHitResult` _outhit))))
    (for (_array_element _array_index) (`self.Itmes`)
      (`/Engine/EditorBlueprintResources/StandardMacros.IsValid` _asbp_item
        (:`Is Valid`
          (bind (_name _stackable _quantity) (break `/Game/Gonjiamerica/Inventory/Blueprints/S_ItemStruct` _array_element))
          (bind (_name_2 _stackable_2 _quantity_2) (break `/Game/Gonjiamerica/Inventory/Blueprints/S_ItemStruct` (`/Game/Gonjiamerica/Inventory/Blueprints/BP_Item.Item` _asbp_item)))
          (bind _returnvalue_2 (+ _quantity _quantity_2))
          (if (and (`KismetTextLibrary.EqualEqual_TextText` _name _name_2) _stackable_2 (<= _returnvalue_2 64))
            (bind (_item_name _item_stackable _item_quantity _item_thumnail) (break `/Game/Gonjiamerica/Inventory/Blueprints/S_ItemStruct` (`/Game/Gonjiamerica/Inventory/Blueprints/BP_Item.Item` _asbp_item)))
            (`KismetArrayLibrary.Array_Set` (`self.Itmes`) _array_index (make `/Game/Gonjiamerica/Inventory/Blueprints/S_ItemStruct` _item_name _item_stackable _returnvalue_2 _item_thumnail))
            (`/Game/Gonjiamerica/Inventory/Widgets/WBP_Inentory.LoadInventory` (`self.Inventorywidget`) self :!label _label)
            (`Actor.K2_DestroyActor` _asbp_item)
            (elif (== _quantity 0)
              (`KismetArrayLibrary.Array_Set` (`self.Itmes`) _array_index (`/Game/Gonjiamerica/Inventory/Blueprints/BP_Item.Item` _asbp_item))
              (goto _label))))))))